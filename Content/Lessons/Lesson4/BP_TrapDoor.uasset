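; BP_TrapDoor is a lesson actor whose Wall rises while something stands in its trigger Box and lowers when it leaves.
; Box begin and end overlap events set the StandingOnButton flag without filtering which actor overlaps.
; Tick nudges the Wall one unit per frame along Z between world heights of about 0 and 300, so its speed depends on frame rate.
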(event `self.ReceiveTick`
  (params (DeltaSeconds :type "Float (single-precision)"))
  (bind _wall (`self.Wall`))
  (bind _wall_2 (`self.Wall`))
  (bind (_returnvalue_x _returnvalue_y _returnvalue_z) (`KismetMathLibrary.BreakVector` (`SceneComponent.K2_GetComponentLocation` _wall_2)))
  (bind (_returnvalue_x_2 _returnvalue_y_2 _returnvalue_z_2) (`KismetMathLibrary.BreakVector` (`SceneComponent.K2_GetComponentLocation` _wall)))
  (if (`self.StandingOnButton`)
    (if (<= _returnvalue_z_2 300.0)
      (`SceneComponent.K2_AddWorldOffset` _wall (`KismetMathLibrary.MakeVector` 0.0 0.0 1.0) false false))
    (elif (>= _returnvalue_z 0.0)
      (`SceneComponent.K2_AddWorldOffset` _wall_2 (`KismetMathLibrary.MakeVector` 0.0 0.0 -1.0) false false))))

(event `self.Box.OnComponentBeginOverlap`
  (params (OverlappedComponent :type "PrimitiveComponent Object Reference") (OtherActor :type "Actor Object Reference") (OtherComp :type "PrimitiveComponent Object Reference") (OtherBodyIndex :type Integer) (bFromSweep :type Boolean) (SweepResult :type "HitResult Structure (by ref)"))
  (set `self.StandingOnButton` true))

(event `self.Box.OnComponentEndOverlap`
  (params (OverlappedComponent :type "PrimitiveComponent Object Reference") (OtherActor :type "Actor Object Reference") (OtherComp :type "PrimitiveComponent Object Reference") (OtherBodyIndex :type Integer))
  (set `self.StandingOnButton` false))

(fn `UserConstructionScript`)