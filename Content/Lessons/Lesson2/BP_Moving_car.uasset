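; BP_Moving_car is a Lesson 2 actor that drives itself around a circular path.
; Each Tick, it adds a fixed-length offset, rotated by the cosine and sine of game time, to its current location without sweep.
; The step ignores delta time, so speed and radius depend on frame rate, and rotation is never set.
; An unconnected SetActorLocation and an unused square-root path formula remain in the graph.
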(event `self.ReceiveTick`
  (params (DeltaSeconds :type "Float (single-precision)"))
  (bind _returnvalue (`KismetSystemLibrary.GetGameTimeInSeconds`))
  (`self.K2_SetActorLocation` (+ (* (`KismetMathLibrary.MakeVector` (`KismetMathLibrary.Cos` _returnvalue) (`KismetMathLibrary.Sin` _returnvalue)) 15) (`self.K2_GetActorLocation`))))

(fn `UserConstructionScript`)