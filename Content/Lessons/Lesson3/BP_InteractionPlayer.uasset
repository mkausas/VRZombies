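; BP_InteractionPlayer is a VR lesson actor for look-to-interact scoring.
; Every tick, a line trace along the VR camera's forward vector places a billboard reticle at the hit point or the ray's far end.
; The Act input repeats that trace, calls InteractMessage on the hit actor and adds the returned value to Score.
; It sends the total to the BP_Scoreboard found at BeginPlay and prints it.
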(event `InputAction|Act`
  (params (Key :type "Key Structure" :default "AnyKey"))
  (:`Pressed`
    (bind (_location _forward_vector) (`/Game/Blueprints/Utility/LayoutVRUtilityFunctions.Get Player VR Camera Properties`))
    (bind (_outhit _returnvalue) (`KismetSystemLibrary.LineTraceSingle` :`Start` _location :`End` (+ _location (* _forward_vector 10000.0)) :`TraceChannel` "TraceTypeQuery1" :`DrawDebugType` "ForDuration"))
    (if _returnvalue
      (bind _score (message `/Game/Lessons/Lesson3/BPI_Interaction.Interact` (`.HitActor` (`GameplayStatics.BreakHitResult` _outhit))))
      (bind _output_get (set `self.Score` (+ _score (`self.Score`))))
      (`/Game/Lessons/Lesson3/BP_Scoreboard.UpdateScore` (`self.Scoreboard`) _output_get)
      (`KismetSystemLibrary.PrintString` (`KismetStringLibrary.Conv_IntToString` _output_get)))))

(event `self.ReceiveBeginPlay`
  (bind _outactors (`GameplayStatics.GetAllActorsOfClass` "/Game/Lessons/Lesson3/BP_Scoreboard.BP_Scoreboard_C"))
  (set `self.Scoreboard` (`KismetArrayLibrary.Array_Get` _outactors)))

(event `self.ReceiveTick`
  (params (DeltaSeconds :type "Float (single-precision)"))
  (bind (_location _forward_vector) (`/Game/Blueprints/Utility/LayoutVRUtilityFunctions.Get Player VR Camera Properties`))
  (bind _returnvalue (+ _location (* _forward_vector 10000.0)))
  (bind (_outhit _returnvalue_2) (`KismetSystemLibrary.LineTraceSingle` :`Start` _location :`End` _returnvalue :`TraceChannel` "TraceTypeQuery1" :`DrawDebugType` "ForDuration"))
  (if _returnvalue_2
    (`SceneComponent.K2_SetWorldLocation` (`self.MaterialBillboard`) (`.Location` (`GameplayStatics.BreakHitResult` _outhit)) false false)
    (else
      (`SceneComponent.K2_SetWorldLocation` (`self.MaterialBillboard`) _returnvalue false false))))

(fn `UserConstructionScript`)