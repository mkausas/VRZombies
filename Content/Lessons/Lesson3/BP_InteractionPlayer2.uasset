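; Lesson 3 interaction Blueprint that lets the player act on a vehicle and three walls through camera gaze and left mouse clicks.
; BeginPlay caches the actors; each press or release line-traces from the VR camera, setting CarDriving when it hits the car, otherwise triggering all walls.
; Tick calls the car's Drive while CarDriving is false, despite the flag's name.
; Tick also traces to position a billboard reticle at the gaze point.
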(event `Key|LeftMouseButton`
  (params (Key :type "Key Structure" :default "AnyKey"))
  (:`Pressed`
    (set `self.CarDriving` false)
    (bind (_location _forward_vector) (`/Game/Blueprints/Utility/LayoutVRUtilityFunctions.Get Player VR Camera Properties` :!label _label))
    (bind _outhit (`KismetSystemLibrary.LineTraceSingle` :`Start` _location :`End` (+ _location (* _forward_vector 10000.0)) :`TraceChannel` "TraceTypeQuery1" :`DrawDebugType` "ForDuration"))
    (bind _returnvalue (== (`.HitActor` (`GameplayStatics.BreakHitResult` _outhit)) (`self.Car`)))
    (if _returnvalue
      (`KismetSystemLibrary.PrintString` "true")
      (set `self.CarDriving` _returnvalue)
      (else
        (`KismetSystemLibrary.PrintString` "false")
        (set `self.CarDriving` _returnvalue)
        (`/Game/Lessons/Lesson3/BP_Wall.Interact` (`self.Wall1`))
        (`/Game/Lessons/Lesson3/BP_Wall.Interact` (`self.Wall2`))
        (`/Game/Lessons/Lesson3/BP_Wall.Interact` (`self.Wall3`)))))
  (:`Released`
    (set `self.CarDriving` true)
    (goto _label)))

(event `self.ReceiveBeginPlay`
  (bind _outactors (`GameplayStatics.GetAllActorsOfClass` "/Game/Lessons/Lesson3/BP_Wall.BP_Wall_C"))
  (set `self.Wall1` (`KismetArrayLibrary.Array_Get` _outactors))
  (set `self.Wall2` (`KismetArrayLibrary.Array_Get` _outactors 1))
  (set `self.Wall3` (`KismetArrayLibrary.Array_Get` _outactors 2))
  (bind _outactors_2 (`GameplayStatics.GetAllActorsOfClass` "/Game/Lessons/Lesson2/BP_Vehicle_Interactive.BP_Vehicle_Interactive_C"))
  (set `self.Car` (`KismetArrayLibrary.Array_Get` _outactors_2)))

(event `self.ReceiveTick`
  (params (DeltaSeconds :type "Float (single-precision)"))
  (if (not (`self.CarDriving`))
    (`/Game/Lessons/Lesson2/BP_Vehicle_Interactive.Drive` (`self.Car`) DeltaSeconds))
  (bind (_location _forward_vector) (`/Game/Blueprints/Utility/LayoutVRUtilityFunctions.Get Player VR Camera Properties`))
  (bind _returnvalue (+ _location (* _forward_vector 10000.0)))
  (bind (_outhit _returnvalue_2) (`KismetSystemLibrary.LineTraceSingle` :`Start` _location :`End` _returnvalue :`TraceChannel` "TraceTypeQuery1" :`DrawDebugType` "ForDuration"))
  (if _returnvalue_2
    (`SceneComponent.K2_SetWorldLocation` (`self.MaterialBillboard`) (`.Location` (`GameplayStatics.BreakHitResult` _outhit)) false false)
    (else
      (`SceneComponent.K2_SetWorldLocation` (`self.MaterialBillboard`) _returnvalue false false))))

(fn `UserConstructionScript`)