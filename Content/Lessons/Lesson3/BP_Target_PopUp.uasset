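; Pop-up target actor that moves vertically after a random startup delay and can be destroyed through interaction.
; On BeginPlay it stores its origin, waits a few seconds, then plays a timeline whose curve scales an upward offset from that origin.
; Interact spawns a particle emitter at the actor's location, destroys the actor and returns a fixed integer to the caller.
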(event `self.ReceiveBeginPlay`
  (set `self.Origin` (`self.K2_GetActorLocation`))
  (`KismetSystemLibrary.Delay` (`KismetMathLibrary.RandomFloatInRange` 2.0 8.0))
  (bind (_direction _data _curve_mycurve) (`Timeline|UpAndDown` :!via `PlayFromStart`)
    (:`Update`
      (`self.K2_SetActorLocation` (+ (`self.Origin`) (* (0.0 0.0 200.0) _curve_mycurve))))))

(fn `Interact`
  (returns (Score :type Integer))
  (`GameplayStatics.SpawnEmitterAtLocation` null (`self.K2_GetActorLocation`))
  (`self.K2_DestroyActor`)
  (return 5))

(fn `UserConstructionScript`)