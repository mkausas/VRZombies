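; BP_Target_ColorChange is a lesson target that randomly switches between blue, green and yellow, with its point value following the color.
; From BeginPlay, ChangeType picks a material and matching Value, where blue is a penalty, then calls itself again after a random delay of a few seconds.
; Interact spawns a small neon explosion, destroys the target and returns the current Value to the caller.
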(event `ChangeType`
  (switch `int` (`KismetMathLibrary.RandomIntegerInRange` 0 2)
    (:`0`
      (`PrimitiveComponent.SetMaterial` (`self.Target`) 0 "/Game/Materials/Props/Combat/Targets/MI_Targets_Blue.MI_Targets_Blue")
      (set `self.Value` -5))
    (:`1`
      (`PrimitiveComponent.SetMaterial` (`self.Target`) 0 "/Game/Materials/Props/Combat/Targets/MI_Targets_Green.MI_Targets_Green")
      (set `self.Value` 5))
    (:`2`
      (`PrimitiveComponent.SetMaterial` (`self.Target`) 0 "/Game/Materials/Props/Combat/Targets/MI_Targets_Yellow.MI_Targets_Yellow")
      (set `self.Value` 10)))
  (`KismetSystemLibrary.Delay` (`KismetMathLibrary.RandomFloatInRange` 2.0 6.0))
  (`self.ChangeType`))

(event `self.ReceiveBeginPlay`
  (`self.ChangeType`))

(fn `Interact`
  (returns (Score :type Integer))
  (`GameplayStatics.SpawnEmitterAtLocation` "/Game/Effects/Particles/Explosion/P_NeonExplosion_Tiny.P_NeonExplosion_Tiny" (`self.K2_GetActorLocation`))
  (`self.K2_DestroyActor`)
  (return (`self.Value`)))

(fn `UserConstructionScript`)