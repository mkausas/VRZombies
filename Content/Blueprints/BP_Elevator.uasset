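; BP_Elevator is an elevator actor that alternately rises and descends by a set height when triggered.
; A capsule overlap notifies MyCharacter on entering and leaving and opens or closes a gate that lets DoAction through.
; DoAction sends the character the leave event, closes all linked doors and starts movement after a short delay.
; Tick moves the actor vertically, stopping and flipping direction at either end.
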(event `self.ReceiveBeginPlay`
  (set `self.DefaultLocation` (`self.K2_GetActorLocation`)))

(event `self.ReceiveActorBeginOverlap`
  (params (OtherActor :type "Actor Object Reference")))

(event `self.ReceiveTick`
  (params (DeltaSeconds :type "Float (single-precision)"))
  (bind _returnvalue (- (.z (`self.K2_GetActorLocation`)) (.z (`self.DefaultLocation`))))
  (if (`self.IsMoveStarted`)
    (`self.K2_SetActorLocation` (`KismetMathLibrary.MakeVector` (.x (`self.K2_GetActorLocation`)) (.y (`self.K2_GetActorLocation`)) (+ (.z (`self.K2_GetActorLocation`)) (* (* DeltaSeconds (`KismetMathLibrary.SelectFloat` 1.0 -1.0 (`self.IsUp`))) (`self.Move Speed`)))))
    (if (`self.IsUp`)
      (if (>= _returnvalue (`self.Move Height`))
        (set `self.IsMoveStarted` false :!label _label)
        (set `self.IsUp` (not (`self.IsUp`))))
      (elif (<= _returnvalue 0.0)
        (goto _label)))))

(event `/Game/Blueprints/BP_I_ActionObject.DoAction`
  (params (Player :type "/Game/Blueprints/MyCharacter Object Reference"))
  (`/Engine/EditorBlueprintResources/StandardMacros.Gate` true :!label _label_2
    (:`Exit`
      (`/Game/Blueprints/MyCharacter.On Elevator Leaved Event` (stale `self.Capsule.OnComponentBeginOverlap` _asmy_character))
      (for _array_element (`self.Doors`)
        (`/Game/Blueprints/BP_Elevator_Doors.Close Doors` _array_element)
        (`KismetSystemLibrary.Delay` 1.0)
        (set `self.IsMoveStarted` true)))))

(event `self.Capsule.OnComponentBeginOverlap`
  (params (OtherActor :type "Actor Object Reference") (OtherComp :type "PrimitiveComponent Object Reference") (OtherBodyIndex :type Integer) (bFromSweep :type Boolean) (SweepResult :type "HitResult Structure (by ref)"))
  (bind _asmy_character (cast `/Game/Blueprints/MyCharacter` OtherActor))
  (`/Game/Blueprints/MyCharacter.On Elevator Entered Event` _asmy_character)
  (goto _label_2 :!via `Open`))

(event `self.Capsule.OnComponentEndOverlap`
  (params (OtherActor :type "Actor Object Reference") (OtherComp :type "PrimitiveComponent Object Reference") (OtherBodyIndex :type Integer))
  (bind _asmy_character (cast `/Game/Blueprints/MyCharacter` OtherActor))
  (`/Game/Blueprints/MyCharacter.On Elevator Leaved Event` _asmy_character)
  (goto _label_2 :!via `Close`))

(fn `UserConstructionScript`)